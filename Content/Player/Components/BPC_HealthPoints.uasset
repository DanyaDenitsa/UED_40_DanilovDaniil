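; Health component in the player folder that tracks hit points for its owner, copying DefaultHP into CurrentHP at BeginPlay.
; IncreaseValue and DecreaseValue adjust CurrentHP through integer property helpers, returning success and broadcasting health changes with a normalized value.
; A decrease that reaches the minimum also broadcasts health reached zero.
; GetIsDead tests DefaultHP, not CurrentHP, against its minimum and fires that same event when true.
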(event EventBeginPlay
  (|SetBy-RefVar (Variables|Default|GetCurrentHP) (Variables|Default|GetDefaultHP)))

(fn GetIsDead
  (bind _defaulthp (Variables|Default|GetDefaultHP))
  (bind (_minvalue _value) (Utilities|Struct|BreakF_PropertyInt _defaulthp))
  (if (<= _value _minvalue)
    (Default|CallOnHealthReachedZero self (Variables|Default|GetCurrentHP))
    (return true)
    (else
      (return false))))

(fn DecreaseValue
  (params (Amount :type Integer))
  (bind _succsess (CallFunction|DecreaseValueInt (Variables|Default|GetCurrentHP) Amount))
  (if _succsess
    (Default|CallOnHealthDecreased self (Variables|Default|GetCurrentHP) (CallFunction|GetNormalizedValue (Variables|Default|GetCurrentHP)))
    (if (CallFunction|ReachedMinValue (Variables|Default|GetCurrentHP))
      (Default|CallOnHealthReachedZero self)
      (return true)
      (else
        (return true)))
    (else
      (return false))))

(fn GetCurrentValue
  (return (Variables|Default|GetCurrentHP)))

(fn IncreaseValue
  (params (Amount :type Integer))
  (bind _succsess (CallFunction|IncreaseValueInt (Variables|Default|GetCurrentHP) Amount))
  (if _succsess
    (Default|CallOnHealthIncreased self (Variables|Default|GetCurrentHP) (CallFunction|GetNormalizedValue (Variables|Default|GetCurrentHP)))
    (return true)
    (else
      (return false))))