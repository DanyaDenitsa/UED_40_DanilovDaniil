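; BP_ItemBase is a base item actor that shows a text label while the player character is within its overlap area.
; Overlap events store the character, toggle the text's visibility and set the interaction-ready and look-at flags.
; While look-at is active, Tick rotates the text to face the player's camera.
; AfterUse destroys the actor; nothing in this Blueprint calls it.
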(event EventBeginPlay
  (Rendering|SetVisibility (Variables|Default|GetTextRender) false false))

(event Collision|EventActorBeginOverlap
  (params (OtherActor :type Actor%20Object%20Reference))
  (bind _asbp_player_character (Utilities|Casting|CastToBP_PlayerCharacter OtherActor))
  (Variables|Default|SetCharacterInBox _asbp_player_character)
  (Rendering|SetVisibility (Variables|Default|GetTextRender) true false)
  (Variables|Default|SetIsReadyToInteract true)
  (Variables|Default|SetIsLookAt true))

(event EventTick
  (params (DeltaSeconds :type Float%20%28single-precision%29))
  (CallFunction|LookingatPlayerCamera))

(event Collision|EventActorEndOverlap
  (params (OtherActor :type Actor%20Object%20Reference))
  (Utilities|Casting|CastToBP_PlayerCharacter OtherActor)
  (Variables|Default|SetCharacterInBox 0)
  (Rendering|SetVisibility (Variables|Default|GetTextRender) false false)
  (Variables|Default|SetIsReadyToInteract false)
  (Variables|Default|SetIsLookAt false))

(fn ConstructionScript)

(fn LookingatPlayerCamera
  (if (Variables|Default|GetIsLookAt)
    (bind _characterinbox (Variables|Default|GetCharacterInBox)
      (:then
        (bind _asbp_player_character (Utilities|Casting|CastToBP_PlayerCharacter _characterinbox))
        (LocalVariables|SetL_CameraLocation (Transformation|GetWorldLocation (Variables|/Game/Player/BP_PlayerCharacter.BP_PlayerCharacter_C|GetCamera _asbp_player_character)))
        (Transformation|SetWorldRotation (Variables|Default|GetTextRender) (Math|Rotator|FindLookatRotation (Transformation|GetWorldLocation (Variables|Default|GetTextRender)) (LocalVariables|GetL_CameraLocation)) false false))
      (:else))))

(fn AfterUse
  (Actor|DestroyActor))