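; Base health pickup actor that heals an overlapping actor.
; Overlap on its Cube component calls ActivatePickUp and destroys the pickup only if that call succeeds.
; The ActivatePickUpEffect function finds the other actor's BPC_HealthPoints component, increases its value by HealPower and returns the result, or false when the component is missing.
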(event OnComponentBeginOverlap(Cube)
  (params (OverlappedComponent :type Primitive%20Component%20Object%20Reference) (OtherActor :type Actor%20Object%20Reference) (OtherComp :type Primitive%20Component%20Object%20Reference) (OtherBodyIndex :type Integer) (bFromSweep :type Boolean) (SweepResult :type Hit%20Result%20Structure%20%28by%20ref%29))
  (bind _success (CallFunction|ActivatePickUp OtherActor))
  (if _success
    (Actor|DestroyActor)))

(event EventBeginPlay
  (|CallParentFunction) ; This node is disabled and will not be called.\nDrag off pins to build functionality.
)

(event Collision|EventActorBeginOverlap
  (params (OtherActor :type Actor%20Object%20Reference))
  (|CallParentFunction OtherActor) ; This node is disabled and will not be called.\nDrag off pins to build functionality.
)

(event EventTick
  (params (DeltaSeconds :type Float%20%28single-precision%29))
  (|CallParentFunction DeltaSeconds) ; This node is disabled and will not be called.\nDrag off pins to build functionality.
)

(fn ConstructionScript
  (|CallParentFunction))

(fn ActivatePickUpEffect
  (params (OtherActor :type Actor%20Object%20Reference))
  (bind _output_get (LocalVariables|SetHealthPoints (Actor|GetComponentbyClass OtherActor "/Game/Player/Components/BPC_HealthPoints.BPC_HealthPoints_C")))
  (Utilities|IsValid _output_get
    (:Is%20Valid
      (bind _succsess (Default|IncreaseValue (LocalVariables|GetHealthPoints) (Variables|Default|GetHealPower)))
      (return _succsess))
    (:Is%20Not%20Valid
      (return false))))