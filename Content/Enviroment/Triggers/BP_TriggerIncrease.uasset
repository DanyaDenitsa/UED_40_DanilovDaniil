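; BP_TriggerIncrease is a trigger that raises the player character's health points when overlapped.
; On begin overlap it runs the parent's handler, then validates the OtherlappedActor variable and casts it to BP_PlayerCharacter.
; A successful cast calls IncreaseValue on the character's BPCHealthPoints component with a fixed amount.
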(event EventBeginPlay
  (|CallParentFunction) ; This node is disabled and will not be called.\nDrag off pins to build functionality.
)

(event Collision|EventActorBeginOverlap
  (params (OtherActor :type Actor%20Object%20Reference))
  (|CallParentFunction OtherActor)
  (bind _otherlappedactor (Variables|Default|GetOtherlappedActor)
    (:then
      (bind _asbp_player_character (Utilities|Casting|CastToBP_PlayerCharacter _otherlappedactor))
      (Default|IncreaseValue (Variables|/Game/Player/BP_PlayerCharacter.BP_PlayerCharacter_C|GetBPC_HealthPoints _asbp_player_character) 50))
    (:else)))

(event EventTick
  (params (DeltaSeconds :type Float%20%28single-precision%29))
  (|CallParentFunction DeltaSeconds) ; This node is disabled and will not be called.\nDrag off pins to build functionality.
)

(fn ConstructionScript
  (|CallParentFunction))