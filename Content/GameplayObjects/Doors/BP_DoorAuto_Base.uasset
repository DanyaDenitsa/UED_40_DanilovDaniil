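; Base automatic swinging door that opens when something enters its trigger volume and closes when it leaves.
; ActivationTrigger overlap events call OpenDoor and CloseDoor, which are not defined in this Blueprint.
; AnimateDoor turns a progress value into motion by interpolating the DoorAncor component's relative yaw from zero to the DoorAncorBase angle.
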(event OnComponentBeginOverlap(ActivationTrigger)
  (params (OverlappedComponent :type Primitive%20Component%20Object%20Reference) (OtherActor :type Actor%20Object%20Reference) (OtherComp :type Primitive%20Component%20Object%20Reference) (OtherBodyIndex :type Integer) (bFromSweep :type Boolean) (SweepResult :type Hit%20Result%20Structure%20%28by%20ref%29))
  (CallFunction|OpenDoor false))

(event OnComponentEndOverlap(ActivationTrigger)
  (params (OverlappedComponent :type Primitive%20Component%20Object%20Reference) (OtherActor :type Actor%20Object%20Reference) (OtherComp :type Primitive%20Component%20Object%20Reference) (OtherBodyIndex :type Integer))
  (CallFunction|CloseDoor false))

(event EventBeginPlay)

(event Collision|EventActorBeginOverlap
  (params (OtherActor :type Actor%20Object%20Reference)))

(event EventTick
  (params (DeltaSeconds :type Float%20%28single-precision%29)))

(fn ConstructionScript
  (|CallParentFunction))

(fn AnimateDoor
  (params (Progress :type Float%20%28double-precision%29))
  (Transformation|SetRelativeRotation (Variables|Default|GetDoorAncor) (Math|Rotator|MakeRotator 0.0 0.0 (Math|Float|Lerp 0.0 (LocalVariables|GetDoorAncorBase) Progress)) false false))