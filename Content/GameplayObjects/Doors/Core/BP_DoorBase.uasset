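; Base door Blueprint that opens and closes, leaving the motion to an empty AnimateDoor function.
; Open and close calls forward to BPC_DoorStateManager, whose transition events play or reverse the DoorAnimation timeline.
; The timeline feeds progress to AnimateDoor and tells the manager when it finishes.
; Construction applies the initial state and pose, scales play rate from AnimationDuration and sets debug text.
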(event OnDoorStateTransitionStart(BPC_DoorStateManager)
  (params (Component :type BPC%20Door%20State%20Manager%20Object%20Reference) (TargetState :type ENUM_DoorState%20Enum :default "NewEnumerator0"))
  (switch Utilities|FlowControl|Switch|SwitchonENUM_DoorState TargetState
    (:NewEnumerator0
      (Components|Timeline|ReversefromEnd (Variables|Default|GetDoorAnimation)))
    (:NewEnumerator1
      (Components|Timeline|PlayfromStart (Variables|Default|GetDoorAnimation)))))

(event OnDoorStateTransitionReversed(BPC_DoorStateManager)
  (params (Component :type BPC%20Door%20State%20Manager%20Object%20Reference) (NewTargetState :type ENUM_DoorState%20Enum :default "NewEnumerator0"))
  (switch Utilities|FlowControl|Switch|SwitchonENUM_DoorState NewTargetState
    (:NewEnumerator0
      (Utilities|String|Reverse (Variables|Default|GetDoorAnimation)))
    (:NewEnumerator1
      (Audio|Components|Audio|Play (Variables|Default|GetDoorAnimation)))))

(fn ConstructionScript
  (if (Utilities|Enum|Equal(Enum) (Variables|Default|GetInitialState) "NewEnumerator3")
    (Variables|Default|SetInitialState "NewEnumerator0"))
  (Default|SetInitialState (Variables|Default|GetBPC_DoorStateManager) (Variables|Default|GetInitialState))
  (CallFunction|AnimateDoor (Utilities|Select :Index (Variables|Default|GetInitialState) :NewEnumerator0 0.0 :NewEnumerator1 1.0 :NewEnumerator2 0.0 :NewEnumerator3 0.0))
  (Components|Timeline|SetPlayRate (Variables|Default|GetDoorAnimation) (Math|Float|SafeDivide 1.0 (Variables|Default|GetAnimationDuration)))
  (CallFunction|DEBUGSetDebugText (Variables|Default|GetInitialState)))

(fn AnimateDoor
  (params (Progress :type Float%20%28double-precision%29)))

(fn DEBUGSetDebugText
  (params (State :type ENUM_DoorState%20Enum :default "NewEnumerator0"))
  (Rendering|Components|TextRender|SetText (Variables|Default|GetDebugText_F) (Utilities|Text|FormatText "============ 
{Name} 
-------------- 
{State} 
--------------" (Utilities|GetDisplayName self) (Utilities|String|EnumtoString State))))

(fn CloseDoor
  (params (TransitImmediatly :type Boolean))
  (bind _success (Default|CloseDoor (Variables|Default|GetBPC_DoorStateManager) TransitImmediatly))
  (return _success))

(fn OpenDoor
  (params (TransitImmediatly :type Boolean))
  (bind _success (Default|OpenDoor (Variables|Default|GetBPC_DoorStateManager) TransitImmediatly))
  (return _success))