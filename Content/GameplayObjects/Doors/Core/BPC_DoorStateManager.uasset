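; BPC_DoorStateManager is a door component that tracks Closed, Opened, Locked and Transition states and announces changes through event dispatchers.
; OpenDoor and CloseDoor feed ChangeState, which either applies the target immediately or enters Transition until FinishTransition commits it.
; ReverseTransition selects on CurrentState, which is always Transition there, so the new target is always Closed.
; SetInitialState sets any non-Transition state without broadcasting.
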(event EventBeginPlay)

(event EventTick
  (params (DeltaSeconds :type Float%20%28single-precision%29)))

(fn OpenDoor
  (params (TransitionImmediatly :type Boolean))
  (if (Utilities|Enum|Equal(Enum) (Variables|Default|GetCurrentState) "NewEnumerator0")
    (bind _success (CallFunction|ChangeState "NewEnumerator1" TransitionImmediatly))
    (return _success)
    (else
      (return false))))

(fn CloseDoor
  (params (TransitionImmediatly :type Boolean))
  (if (Utilities|Enum|Equal(Enum) (Variables|Default|GetCurrentState) "NewEnumerator1")
    (bind _success (CallFunction|ChangeState "NewEnumerator0" TransitionImmediatly))
    (return _success)
    (else
      (return false))))

(fn ChangeState
  (params (NewState :type ENUM_DoorState%20Enum :default "NewEnumerator0") (TransitImmediatly :type Boolean))
  (if (and (Utilities|Enum|NotEqual(Enum) NewState (Variables|Default|GetCurrentState)) (Utilities|Enum|NotEqual(Enum) NewState "NewEnumerator3"))
    (Variables|Default|SetTargetState NewState)
    (Variables|Default|SetPreviousState (Variables|Default|GetCurrentState))
    (Variables|Default|SetCurrentState (select TransitImmediatly (Variables|Default|GetTargetState) "NewEnumerator3"))
    (Default|CallOnDoorStateChanged self (Variables|Default|GetCurrentState))
    (if TransitImmediatly
      _
      (else
        (Default|CallOnDoorStateTransitionStart self (Variables|Default|GetTargetState))))
    (return true)
    (else
      (return false))))

(fn FinishTransition
  (if (Utilities|Enum|Equal(Enum) (Variables|Default|GetCurrentState) "NewEnumerator3")
    (bind _success (CallFunction|ChangeState (Variables|Default|GetTargetState) true))
    (return _success)
    (else
      (return false))))

(fn SetInitialState
  (params (NewState :type ENUM_DoorState%20Enum :default "NewEnumerator0"))
  (if (Utilities|Enum|NotEqual(Enum) NewState "NewEnumerator3")
    (Variables|Default|SetCurrentState NewState)
    (return)
    (else
      (return))))

(fn ReverseTransition
  (if (Utilities|Enum|Equal(Enum) (Variables|Default|GetCurrentState) "NewEnumerator3")
    (bind _output_get (Variables|Default|SetTargetState (Utilities|Select :Index (Variables|Default|GetCurrentState) :NewEnumerator0 "NewEnumerator1" :NewEnumerator1 "NewEnumerator0" :NewEnumerator2 "NewEnumerator0" :NewEnumerator3 "NewEnumerator0")))
    (Default|CallOnDoorStateTransitionReversed self _output_get)
    (return true)
    (else
      (return false))))