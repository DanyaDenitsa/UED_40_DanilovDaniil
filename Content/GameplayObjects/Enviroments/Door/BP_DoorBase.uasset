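; Base door Blueprint that swings open when a BP_PlayerCharacter enters its box and attempts closing on exit.
; A timeline scales DoorAngle into DoorRotator yaw, setting InProcess during updates.
; Open and close both require IsClose, and the finish handler skips InProcess, so the state can stick there and block closing.
; The construction script applies DoorAngle as a Z location offset when IsOpen, rather than rotation.
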(event OnComponentBeginOverlap(Box)
  (params (OverlappedComponent :type Primitive%20Component%20Object%20Reference) (OtherActor :type Actor%20Object%20Reference) (OtherComp :type Primitive%20Component%20Object%20Reference) (OtherBodyIndex :type Integer) (bFromSweep :type Boolean) (SweepResult :type Hit%20Result%20Structure%20%28by%20ref%29))
  (Utilities|Casting|CastToBP_PlayerCharacter OtherActor)
  (CallFunction|OpenDoor))

(event OnComponentEndOverlap(Box)
  (params (OverlappedComponent :type Primitive%20Component%20Object%20Reference) (OtherActor :type Actor%20Object%20Reference) (OtherComp :type Primitive%20Component%20Object%20Reference) (OtherBodyIndex :type Integer))
  (Utilities|Casting|CastToBP_PlayerCharacter OtherActor)
  (CallFunction|CloseDoor))

(event Custom|OpenDoor
  (if (Utilities|Enum|Equal(Enum) (Variables|Default|GetDoorStates) "NewEnumerator1")
    (bind (_direction _openprogression) (Timeline|DoorTimeline PlayFromStart)
      (:Update
        (Variables|Default|SetDoorStates "NewEnumerator3")
        (Transformation|SetRelativeRotation (Variables|Default|GetDoorRotator) (Math|Rotator|MakeRotator 0.0 0.0 (* (Variables|Default|GetDoorAngle) _openprogression)) false false))
      (:Finished
        (if (Utilities|Enum|NotEqual(Enum) (Variables|Default|GetDoorStates) "NewEnumerator3")
          (switch Utilities|FlowControl|Switch|SwitchonETimelineDirection _direction
            (:Forward
              (bind _output_get (Variables|Default|SetDoorStates "NewEnumerator0"))
              (Development|PrintString "Hello" true false "(R=0.000000,G=0.660000,B=1.000000,A=1.000000)" 2.0 (Utilities|Name|EnumtoName _output_get)))
            (:Backward
              (bind _output_get_2 (Variables|Default|SetDoorStates "NewEnumerator1"))
              (Development|PrintString "Hello" true false "(R=0.000000,G=0.660000,B=1.000000,A=1.000000)" 2.0 (Utilities|Name|EnumtoName _output_get_2)))))))))

(event Custom|CloseDoor
  (if (Utilities|Enum|Equal(Enum) (Variables|Default|GetDoorStates) "NewEnumerator1")
    (bind (_direction _openprogression) (Timeline|DoorTimeline ReverseFromEnd)
      (:Update
        (Variables|Default|SetDoorStates "NewEnumerator3")
        (Transformation|SetRelativeRotation (Variables|Default|GetDoorRotator) (Math|Rotator|MakeRotator 0.0 0.0 (* (Variables|Default|GetDoorAngle) _openprogression)) false false))
      (:Finished
        (if (Utilities|Enum|NotEqual(Enum) (Variables|Default|GetDoorStates) "NewEnumerator3")
          (switch Utilities|FlowControl|Switch|SwitchonETimelineDirection _direction
            (:Forward
              (bind _output_get (Variables|Default|SetDoorStates "NewEnumerator0"))
              (Development|PrintString "Hello" true false "(R=0.000000,G=0.660000,B=1.000000,A=1.000000)" 2.0 (Utilities|Name|EnumtoName _output_get)))
            (:Backward
              (bind _output_get_2 (Variables|Default|SetDoorStates "NewEnumerator1"))
              (Development|PrintString "Hello" true false "(R=0.000000,G=0.660000,B=1.000000,A=1.000000)" 2.0 (Utilities|Name|EnumtoName _output_get_2)))))))))

(event EventBeginPlay)

(event Collision|EventActorBeginOverlap
  (params (OtherActor :type Actor%20Object%20Reference)))

(event EventTick
  (params (DeltaSeconds :type Float%20%28single-precision%29)))

(fn ConstructionScript
  (Transformation|AddRelativeLocation (Variables|Default|GetDoorRotator) (Math|Vector|MakeVector 0.0 0.0 (Math|Float|SelectFloat (Variables|Default|GetDoorAngle) 0.0 (Utilities|Enum|Equal(Enum) (Variables|Default|GetDoorStates) "NewEnumerator0"))) false false))

(fn SetState
  (params (DoorStates :type ENUM_DoorStates%20Enum :default "NewEnumerator0"))
  (switch Utilities|FlowControl|Switch|SwitchonENUM_DoorStates DoorStates
    (:NewEnumerator0
      (CallFunction|OpenDoor))
    (:NewEnumerator1
      (CallFunction|CloseDoor))
    (:NewEnumerator2
      (CallFunction|IsBlocked))
    (:NewEnumerator3
      (CallFunction|InProcess))))

(fn IsOpen
  (if (Utilities|Enum|Equal(Enum) (Variables|Default|GetDoorStates) "NewEnumerator0")
    (return true)
    (else
      (return false))))

(fn IsClose
  (if (Utilities|Enum|Equal(Enum) (Variables|Default|GetDoorStates) "NewEnumerator1")
    (return true)
    (else
      (return false))))

(fn IsBlocked
  (if (Utilities|Enum|Equal(Enum) (Variables|Default|GetDoorStates) "NewEnumerator2")
    (return true)
    (else
      (return false))))

(fn InProcess
  (return false))